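; Player character for samurai melee combat, with equip toggle, run, directional dodge, defense stance and target lock.
; Montages drive non-repeating random attacks, with a reset event for chaining, while a sphere trace sends damage messages.
; Incoming damage is ignored mid-dodge, otherwise choosing block, guard-break or hit reactions by defense and attack type.
; Lock-on picks the nearest BP_EnemyAI in range, and Tick interpolates control rotation toward it.
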(event Custom|ResetAttackMontage
  ;[1 1 1] Attack (Combo)
  ;;[1 1 1] Attack animation cancel (smooth combo)
  (Variables|Default|SetAttackMontagePlay false)
  ;;[1 1 1] Attack into quick defense
  (if (Variables|Default|GetDefense)
    (Animation|StopAnimMontage (Utilities|Array|Get(acopy) (Variables|Default|GetAttack%20Montage%20to%20Play) (Variables|Default|GetCurrent%20Attack%20Int)))))

(event Custom|AttackSphere
  (bind _arrow1 (Variables|Default|GetArrow1))
  (bind _returnvalue (Transformation|GetWorldLocation _arrow1))
  ;[1 1 1] Hit area
  (bind (_outhits _returnvalue_2) (Collision|MultiSphereTraceByChannel _returnvalue (+ _returnvalue (* (Math|Vector|GetForwardVector _arrow1) 1.5e+02)) 5e+01 "TraceTypeQuery1" false 0 "None"))
  (if _returnvalue_2
    (for _array_element _outhits
      (Class|BPIDamage|Damage(Message) (.HitActor (Collision|BreakHitResult _array_element)) (Variables|Default|GetAttackDamage) false))))

(event EventTick
  (params (DeltaSeconds :type Float%20%28single-precision%29))
  ;[1 0.05882 0.05882] Event Tick
  (Utilities|FlowControl|Sequence
    (:then_0
      (|Cameramoveorientation))
    (:then_1
      (|Orientationfixduringattackcombo))
    (:then_2
      (|Cameratargetlockorientation))))

(event EventDamage
  (params (Damage :type Float%20%28double-precision%29) (SpecialAttack :type Boolean))
  ;[1 1 1] Damage
  (Variables|Default|SetAttackMontagePlay false)
  (if (not (Variables|Default|GetDodgeMontagePlay))
    (Variables|Default|SetHitMontagePlay true)
    (if SpecialAttack ; special attack ?
      (Utilities|FlowControl|Sequence ; Get hit by special attack
        (:then_0
          ;;[1 1 1] Get hit by normal attack
          (|DamageVFX&SFX :!label _label))
        (:then_1
          (if (Variables|Default|GetDefense) ; break defense or get hit
            ;;[1 1 1] Break defense
            (Animation|Montage|MontagePlay (Components|SkeletalMesh|GetAnimInstance (Variables|Character|GetMesh)) "/Game/GhostSamurai_Katana/GhostSamurai_Katana/Animation/Defense/Root/GhostSamurai_DefenseR_Broken_Root_Montage.GhostSamurai_DefenseR_Broken_Root_Montage" 1.0 "MontageLength" 0.0 true)
            (Utilities|FlowControl|Delay 0.5)
            (Variables|Default|SetHitMontagePlay false)
            (else
              ;;[1 1 1] get hit by special attack
              (Animation|Montage|MontagePlay (Components|SkeletalMesh|GetAnimInstance (Variables|Character|GetMesh)) "/Game/GhostSamurai_Katana/GhostSamurai_Katana/Animation/Apose/Hit/Root/GhostSamurai_APose_Large_Hit_Root_Montage.GhostSamurai_APose_Large_Hit_Root_Montage" 1.0 "MontageLength" 0.0 true)
              (Utilities|FlowControl|Delay 0.5)
              (Variables|Default|SetHitMontagePlay false)))))
      (elif (Variables|Default|GetDefense) ; block or get hit
        ;;[1 1 1] Block
        (|Blockfeedback
          (:NewParam2
            (Animation|Montage|MontagePlay (Components|SkeletalMesh|GetAnimInstance (Variables|Character|GetMesh)) "/Game/GhostSamurai_Katana/GhostSamurai_Katana/Animation/Defense/Root/GhostSamurai_DefenseR_Hit01_Root_Montage.GhostSamurai_DefenseR_Hit01_Root_Montage" 1.0 "MontageLength" 0.0 true)
            (Utilities|FlowControl|Delay 0.3)
            (Variables|Default|SetHitMontagePlay false)))
        (else
          (Utilities|FlowControl|Sequence
            (:then_0
              (Animation|Montage|MontagePlay (Components|SkeletalMesh|GetAnimInstance (Variables|Character|GetMesh)) "/Game/GhostSamurai_Katana/GhostSamurai_Katana/Animation/Apose/Hit/Root/GhostSamurai_APose_Hit_F_Root_Montage.GhostSamurai_APose_Hit_F_Root_Montage" 1.0 "MontageLength" 0.0 true)
              (Utilities|FlowControl|Delay 0.5)
              (Variables|Default|SetHitMontagePlay false))
            (:then_1
              (|CameraShake
                (:NewParam2
                  (goto _label))))))))))

(event EventBeginPlay
  ;[1 0.05882 0.05882] Event Bgein Play
  (Utilities|FlowControl|Sequence
    (:then_0
      (|BeginPlayFindenemytolockon))))

(event Input|ActionEvents|InputActionWalk/Run
  (params (Key :type Key%20Structure :default "None"))
  ;[1 1 1] Run
  (:Pressed
    (if (not (Variables|Default|GetDefense))
      (Variables|Default|SetRun true)
      (bind _runvalue (Timeline|Run_Timeline Play)
        (:Update
          (Variables|/Script/Engine.CharacterMovementComponent|SetMaxWalkSpeed (Variables|Character|GetCharacterMovement) _runvalue)))))
  (:Released
    (if (not (Variables|Default|GetDefense))
      (bind _runvalue_2 (Timeline|Timeline Reverse)
        (:Update
          (Variables|/Script/Engine.CharacterMovementComponent|SetMaxWalkSpeed (Variables|Character|GetCharacterMovement) _runvalue_2))
        (:Finished
          (Variables|Default|SetRun false))))))

(event Input|ActionEvents|InputActionDefense
  (params (Key :type Key%20Structure :default "None"))
  ;[1 1 1] Defense Stance
  (:Pressed
    (if (Variables|Default|GetRun)
      (Utilities|FlowControl|Sequence
        (:then_0
          ;[1 1 1] Run
          (bind _runvalue (Timeline|Timeline Reverse)
            (:Update
              (Variables|/Script/Engine.CharacterMovementComponent|SetMaxWalkSpeed (Variables|Character|GetCharacterMovement) _runvalue))
            (:Finished
              (Variables|Default|SetRun false))))
        (:then_1
          (Variables|Default|SetDefense true :!label _label)))
      (else
        (goto _label))))
  (:Released
    (Variables|Default|SetDefense false)))

(event Input|ActionEvents|InputActionDodge
  (params (Key :type Key%20Structure :default "None"))
  (bind _returnvalue (Input|AxisValues|GetMoveForward))
  (bind _returnvalue_2 (Input|AxisValues|GetMoveRight))
  ;[1 1 1] Dodge (temp)
  (:Pressed
    (if (and (Math|Boolean|NORBoolean (Variables|Default|GetDodgeMontagePlay) (Variables|Default|GetAttackMontagePlay)) (Variables|Default|GetEquipped))
      (Utilities|FlowControl|Sequence
        (:then_0
          (Variables|Default|SetDodgeMontagePlay true)
          (if (!= _returnvalue 0.0)
            (if (> _returnvalue 0.0)
              ;;[1 1 1] Roll Forward
              (Animation|Montage|PlayMontage (Variables|Character|GetMesh) "/Game/GhostSamurai_Katana/GhostSamurai_Katana/Animation/Apose/Dodge/Root/GhostSamurai_APose_Dodge_F_Root_Montage.GhostSamurai_APose_Dodge_F_Root_Montage" 1.2
                (:OnCompleted
                  (Variables|Default|SetDodgeMontagePlay false)))
              (else
                ;;[1 1 1] Roll Back
                (Animation|Montage|PlayMontage (Variables|Character|GetMesh) "/Game/GhostSamurai_Katana/GhostSamurai_Katana/Animation/Apose/Dodge/Root/GhostSamurai_APose_Dodge_B_Root_Montage.GhostSamurai_APose_Dodge_B_Root_Montage" 1.2 :!label _label
                  (:OnCompleted
                    (Variables|Default|SetDodgeMontagePlay false)))))
            (elif (!= _returnvalue_2 0.0)
              (if (> _returnvalue_2 0.0)
                ;;[1 1 1] Roll Right
                (Animation|Montage|PlayMontage (Variables|Character|GetMesh) "/Game/GhostSamurai_Katana/GhostSamurai_Katana/Animation/Apose/Dodge/Root/GhostSamurai_APose_Dodge_R_Root_Montage.GhostSamurai_APose_Dodge_R_Root_Montage" 1.2
                  (:OnCompleted
                    (Variables|Default|SetDodgeMontagePlay false)))
                (else
                  ;;[1 1 1] Roll Left
                  (Animation|Montage|PlayMontage (Variables|Character|GetMesh) "/Game/GhostSamurai_Katana/GhostSamurai_Katana/Animation/Apose/Dodge/Root/GhostSamurai_APose_Dodge_L_Root_Montage.GhostSamurai_APose_Dodge_L_Root_Montage" 1.2
                    (:OnCompleted
                      (Variables|Default|SetDodgeMontagePlay false)))))
              (else
                (goto _label)))))
        (:then_1
          (|CameraShake_2))))))

(event Input|ActionEvents|InputActionAttack
  (params (Key :type Key%20Structure :default "None"))
  ;[1 1 1] Attack (Combo)
  (:Pressed
    (if (and (Math|Boolean|NORBoolean (Variables|Default|GetDodgeMontagePlay) (Variables|Default|GetAttackMontagePlay)) (Variables|Default|GetEquipped))
      (Utilities|FlowControl|Sequence
        (:then_0
          (Variables|Default|SetAttackMontagePlay true)
          ;;[1 1 1] Random attack different from previous
          (Variables|Default|SetCount%20Attack%20Int 0)
          (while (or (== (Variables|Default|GetPrevious%20Attack%20Int) (Variables|Default|GetCurrent%20Attack%20Int)) (== 5 (Variables|Default|GetCount%20Attack%20Int)))
            (Variables|Default|SetCurrent%20Attack%20Int (Math|Random|RandomInteger 4))
            (Math|Integer|IncrementInt (Variables|Default|GetCount%20Attack%20Int)))
          (Variables|Default|SetPrevious%20Attack%20Int (Variables|Default|GetCurrent%20Attack%20Int))
          (Animation|Montage|PlayMontage (Variables|Character|GetMesh) (Utilities|Array|Get(acopy) (Variables|Default|GetAttack%20Montage%20to%20Play) (Variables|Default|GetCurrent%20Attack%20Int))
            (:OnCompleted
              (Variables|Default|SetAttackMontagePlay false))))
        (:then_1
          (|CameraShake_2_2))
        (:then_2
          (Variables|Default|SetDefense false))))))

(event Input|ActionEvents|InputActionTargetLock
  (params (Key :type Key%20Structure :default "None"))
  ;[1 1 1] Target Lock
  (:Pressed
    (Utilities|FlowControl|FlipFlop
      (:A
        (Variables|Default|SetLock true)
        (|Findenemytolockon))
      (:B
        (Variables|Default|SetLock false)))))

(event Input|AxisEvents|InputAxisMouseX
  (params (AxisValue :type Float%20%28single-precision%29))
  ;[0 0.2824 1] Camera Rotation / Look
  (if (not (Variables|Default|GetLock))
    (Pawn|Input|AddControllerYawInput AxisValue)))

(event Input|AxisEvents|InputAxisMouseY
  (params (AxisValue :type Float%20%28single-precision%29))
  ;[0 0.2824 1] Camera Rotation / Look
  (if (not (Variables|Default|GetLock))
    (Pawn|Input|AddControllerPitchInput AxisValue)))

(event Input|AxisEvents|InputAxisMoveForward
  (params (AxisValue :type Float%20%28single-precision%29))
  ;[0 0.2824 1] Camera Rotation / Look
  (Pawn|Input|AddMovementInput (Math|Vector|GetForwardVector (Math|Rotator|MakeRotator 0.0 0.0 (.Yaw (Math|Rotator|BreakRotator (Pawn|GetControlRotation :!class /Script/Engine.Pawn))))) AxisValue false))

(event Input|AxisEvents|InputAxisMoveRight
  (params (AxisValue :type Float%20%28single-precision%29))
  ;[0 0.2824 1] Camera Rotation / Look
  (Pawn|Input|AddMovementInput (Math|Vector|GetRightVector (Math|Rotator|MakeRotator 0.0 0.0 (.Yaw (Math|Rotator|BreakRotator (Pawn|GetControlRotation :!class /Script/Engine.Pawn))))) AxisValue false))

(event Input|KeyboardEvents|1
  (params (Key :type Key%20Structure :default "None"))
  (bind _mesh (Variables|Character|GetMesh))
  ;[1 1 1] Equip  /Unequip
  (:Pressed
    (if (Variables|Default|GetEquipped)
      (Animation|Montage|PlayMontage _mesh "/Game/GhostSamurai_Katana/GhostSamurai_Katana/Animation/Common/Root/GhostSamurai_APose_Equip02_Root_Montage_Inverse.GhostSamurai_APose_Equip02_Root_Montage_Inverse"
        (:OnCompleted
          (Variables|Default|SetEquipped false)))
      (else
        (Animation|Montage|PlayMontage _mesh "/Game/GhostSamurai_Katana/GhostSamurai_Katana/Animation/Common/Root/GhostSamurai_APose_Equip02_Root_Montage.GhostSamurai_APose_Equip02_Root_Montage"
          (:then
            (Utilities|FlowControl|Delay 0.9)
            (Class|BPIReadytoFight|Ready(Message) (Variables|Default|GetTarget)))
          (:OnCompleted
            (Variables|Default|SetEquipped true)))))))

(fn ConstructionScript)

(fn CalculateLastInput
  (bind _charactermovement (Variables|Character|GetCharacterMovement))
  (bind _returnvalue (Pawn|Components|PawnMovement|GetLastInputVector _charactermovement))
  (Variables|Default|SetLast%20Input _returnvalue)
  (bind _output_get (Variables|Default|SetValid%20Input (Utilities|Operators|NotEqual(!=) :A _returnvalue)))
  (if _output_get
    (Variables|Default|SetLast%20Rotation (Math|Conversions|RotationFromXVector _returnvalue))))

(fn RinterptoRotation
  (params (Is%20Interp :type Boolean))
  (if Is%20Interp
    (Transformation|SetActorRotation (Math|Interpolation|RInterpTo (Transformation|GetActorRotation) (Variables|Default|GetLast%20Rotation) (Utilities|Time|GetWorldDeltaSeconds) 15.0))))