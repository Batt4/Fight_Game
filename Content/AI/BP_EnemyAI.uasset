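; Enemy samurai AI character that runs a behavior tree and fights a BP_BaseRoll target, sharing state through the blackboard.
; Looping randomized timers trigger defense, strafing and dash or jump specials, which lerp toward the target with timelines.
; Tick turns it to face the target and applies sideways input.
; Attacks randomly dodge or pick varied montages, sphere traces deal damage, and hit reactions depend on dodge and defense state.
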(event Custom|Attack
  ;[1 1 1] Attack
  (if (not (or (Variables|Default|GetHitMontagePlay) (Variables|Default|GetAttackMontage)))
    (Variables|Default|SetAttackMontage true)
    ;;[1 1 1] dont like this kind of logic
    (if (== (Math|Random|RandomInteger 6) 0)
      ;;[1 1 1] Dodge backwards
      (Variables|Default|SetDodgeMontagePlay true)
      (Animation|Montage|PlayMontage (Variables|Character|GetMesh) "/Game/GhostSamurai_Katana/GhostSamurai_Katana/Animation/Apose/Dodge/Root/GhostSamurai_APose_Dodge_B_Root_Montage.GhostSamurai_APose_Dodge_B_Root_Montage"
        (:OnCompleted
          (Variables|Default|SetDodgeMontagePlay false)))
      (else
        ;;[1 1 1] Random attack different from previous
        (Variables|Default|SetCount%20Attack%20Int 0)
        (while (or (== (Variables|Default|GetPrevious%20Attack%20Int) (Variables|Default|GetCurrent%20Attack%20Int)) (== 5 (Variables|Default|GetCount%20Attack%20Int)))
          (Variables|Default|SetCurrent%20Attack%20Int (Math|Random|RandomInteger 4))
          (Math|Integer|IncrementInt (Variables|Default|GetCount%20Attack%20Int)))
        (bind _output_get (Variables|Default|SetPrevious%20Attack%20Int (Variables|Default|GetCurrent%20Attack%20Int)))
        (Animation|Montage|MontagePlay (Components|SkeletalMesh|GetAnimInstance (Variables|Character|GetMesh)) (Utilities|Array|Get(acopy) (Variables|Default|GetAttack%20Montage%20to%20Play) _output_get) 1.0 "MontageLength" 0.0 true)))))

(event Custom|AttackSphere
  (params (SpecialAttack :type Boolean))
  (bind _arrow1 (Variables|Default|GetArrow1))
  (bind _returnvalue (Transformation|GetWorldLocation _arrow1))
  ;[1 1 1] Hit area (AttackSphere)
  (bind (_outhits _returnvalue_2) (Collision|MultiSphereTraceByChannel _returnvalue (+ _returnvalue (* (Math|Vector|GetForwardVector _arrow1) 1.5e+02)) 5e+01 "TraceTypeQuery1" false 0 "None"))
  (if _returnvalue_2
    (for _array_element _outhits
      (Class|BPIDamage|Damage(Message) (.HitActor (Collision|BreakHitResult _array_element)) (Variables|Default|GetAttackDamage) SpecialAttack))))

(event Custom|ResetAttack
  ;[1 1 1] Attack
  (Variables|Default|SetAttackMontage false)
  (Variables|Default|SetDodgeMontagePlay false))

(event Custom|SetDefense
  ;[1 0.06771 0.06771] Event Begin Play
  ;;[1 1 1] Defense //// wtf random defense stance - change the defense system into sth with a brain
  (CallFunction|StopRunning)
  (Variables|Default|SetDefense true)
  (Utilities|FlowControl|Delay (Math|Random|RandomFloatinRange 3.0 8.0))
  (Variables|Default|SetDefense false))

(event Custom|SetStrafe
  ;[1 0.06771 0.06771] Event Begin Play
  ;;[1 1 1] Strafe / Walk sideways
  (bind _output_get (Variables|Default|SetStrafe true))
  (AI|Components|Blackboard|SetValueasBool (AI|GetBlackboard 0) (Utilities|Name|MakeLiteralName "Strafe") _output_get))

(event Custom|Run
  ;[1 1 1] Run
  (Variables|Default|SetRunning true)
  (bind (_direction _runvalue) (Timeline|Timeline Play)
    (:Update
      (Variables|/Script/Engine.CharacterMovementComponent|SetMaxWalkSpeed (Variables|Character|GetCharacterMovement) _runvalue)
      (AI|Components|Blackboard|SetValueasBool (AI|GetBlackboard 0) (Utilities|Name|MakeLiteralName "Running") (Variables|Default|GetRunning) :!label _label))
    (:Finished
      (if (Utilities|Enum|Equal(Enum) _direction "Backward")
        (Variables|Default|SetRunning false)
        (goto _label)))))

(event Custom|StopRunning
  ;[1 1 1] Run
  (bind (_direction _runvalue) (Timeline|Timeline Reverse)
    (:Update
      (Variables|/Script/Engine.CharacterMovementComponent|SetMaxWalkSpeed (Variables|Character|GetCharacterMovement) _runvalue)
      (AI|Components|Blackboard|SetValueasBool (AI|GetBlackboard 0) (Utilities|Name|MakeLiteralName "Running") (Variables|Default|GetRunning) :!label _label))
    (:Finished
      (if (Utilities|Enum|Equal(Enum) _direction "Backward")
        (Variables|Default|SetRunning false)
        (goto _label)))))

(event Custom|JumpAttack
  ;[1 1 1] Special attack
  (Variables|Default|SetAttackMontage true))

(event Custom|SpecialAttack
  (bind _returnvalue (Transformation|GetActorForwardVector))
  (bind _target (Variables|Default|GetTarget))
  (bind _target_2 (Variables|Default|GetTarget))
  (bind _target_3 (Variables|Default|GetTarget))
  (bind _returnvalue_2 (Transformation|GetActorLocation _target))
  (bind _returnvalue_3 (Transformation|GetActorLocation _target_2))
  (bind _returnvalue_4 (Transformation|GetActorLocation _target_3))
  ;[1 1 1] Special attack
  (Variables|Default|SetAttackMontage true)
  (if (Math|Random|RandomBool)
    ;;[1 1 1] DashAttack
    (Animation|Montage|MontagePlay (Components|SkeletalMesh|GetAnimInstance (Variables|Character|GetMesh)) "/Game/GhostSamurai_Katana/GhostSamurai_Katana/Animation/Apose/Attack/Root/GhostSamurai_APose_SPAttack01_Root_Montage.GhostSamurai_APose_SPAttack01_Root_Montage" 1.0 "MontageLength" 0.0 true)
    (Utilities|FlowControl|Delay 0.45)
    (Variables|Default|SetTargetLocation (Math|Vector|MakeVector (+ (.x _returnvalue_3) 1e+02) (.y _returnvalue_3) (.z _returnvalue_3)))
    (Utilities|FlowControl|Delay 0.45)
    (bind _alpha (Timeline|SpecialAttack_Timeline PlayFromStart)
      (:Update
        (Transformation|SetActorLocation (Math|Vector|Lerp(Vector) (Transformation|GetActorLocation) (Variables|Default|GetTargetLocation) _alpha) false false)))
    (else
      ;;[1 1 1] Jump attack
      (Animation|Montage|MontagePlay (Components|SkeletalMesh|GetAnimInstance (Variables|Character|GetMesh)) "/Game/GhostSamurai_Katana/GhostSamurai_Katana/Animation/Apose/Attack/Root/GhostSamurai_APose_JumpAttack02_Root_Montage.GhostSamurai_APose_JumpAttack02_Root_Montage" 1.0 "MontageLength" 0.0 true)
      (Character|LaunchCharacter (Math|Vector|MakeVector (.x _returnvalue) (.y _returnvalue) (Variables|Default|GetJumpAttackHeight)) true true)
      (Utilities|FlowControl|Delay 0.2)
      (Variables|Default|SetTargetLocation (Math|Vector|MakeVector (+ (.x _returnvalue_4) -1.5e+02) (.y _returnvalue_4) (.z _returnvalue_4)))
      (Utilities|FlowControl|Sequence
        (:then_0
          (bind _alpha_2 (Timeline|Timeline_0 PlayFromStart)
            (:Update
              (Transformation|SetActorLocation (Math|Vector|Lerp(Vector) (Transformation|GetActorLocation) (Variables|Default|GetTargetLocation) _alpha_2) false false))))
        (:then_1
          (Utilities|FlowControl|Delay 0.2)
          (Variables|Default|SetTargetLocation (Math|Vector|MakeVector (+ (.x _returnvalue_2) 1e+02) (.y _returnvalue_2) (.z _returnvalue_2))))))))

(event Custom|DashAttack
  (bind _target (Variables|Default|GetTarget))
  (bind _returnvalue (Transformation|GetActorLocation _target))
  ;[1 1 1] Special attack
  (Variables|Default|SetAttackMontage true)
  ;;[1 1 1] DashAttack
  (Animation|Montage|MontagePlay (Components|SkeletalMesh|GetAnimInstance (Variables|Character|GetMesh)) "/Game/GhostSamurai_Katana/GhostSamurai_Katana/Animation/Apose/Attack/Root/GhostSamurai_APose_SPAttack01_Root_Montage.GhostSamurai_APose_SPAttack01_Root_Montage" 1.0 "MontageLength" 0.0 true)
  (Utilities|FlowControl|Delay 0.45)
  (Variables|Default|SetTargetLocation (Math|Vector|MakeVector (+ (.x _returnvalue) 1e+02) (.y _returnvalue) (.z _returnvalue)))
  (Utilities|FlowControl|Delay 0.45)
  (bind _alpha (Timeline|SpecialAttack_Timeline PlayFromStart)
    (:Update
      (Transformation|SetActorLocation (Math|Vector|Lerp(Vector) (Transformation|GetActorLocation) (Variables|Default|GetTargetLocation) _alpha) false false))))

(event EventDamage
  (params (Damage :type Float%20%28double-precision%29) (SpecialAttack :type Boolean))
  ;[1 1 1] Damage
  (Variables|Default|SetAttackMontage false)
  (if (not (Variables|Default|GetDodgeMontagePlay))
    (Variables|Default|SetHitMontagePlay true)
    (if (not SpecialAttack)
      (if (Variables|Default|GetDefense)
        (|Blockfeedback_2
          (:NewParam2
            (Animation|Montage|MontagePlay (Components|SkeletalMesh|GetAnimInstance (Variables|Character|GetMesh)) "/Game/GhostSamurai_Katana/GhostSamurai_Katana/Animation/Defense/Root/GhostSamurai_DefenseR_Hit01_Root_Montage.GhostSamurai_DefenseR_Hit01_Root_Montage" 1.0 "MontageLength" 0.0 true)
            (Utilities|FlowControl|Delay 0.3)
            (Variables|Default|SetHitMontagePlay false)))
        (else
          (Animation|Montage|MontagePlay (Components|SkeletalMesh|GetAnimInstance (Variables|Character|GetMesh)) "/Game/GhostSamurai_Katana/GhostSamurai_Katana/Animation/Apose/Hit/Root/GhostSamurai_APose_Hit_F_Root_Montage.GhostSamurai_APose_Hit_F_Root_Montage" 1.0 "MontageLength" 0.0 true)
          (Utilities|FlowControl|Delay 0.5)
          (Variables|Default|SetHitMontagePlay false))))))

(event EventTick
  (params (DeltaSeconds :type Float%20%28single-precision%29))
  ;[1 0.07812 0.07812] Event Tick
  ;;[1 1 1] Move Sideways
  (Transformation|SetActorRotation (Math|Interpolation|RInterpTo (Transformation|GetActorRotation) (Math|Rotator|FindLookatRotation (Transformation|GetActorLocation) (Transformation|GetActorLocation (Variables|Default|GetTarget))) (Utilities|Time|GetWorldDeltaSeconds) 25.0))
  (Pawn|Input|AddMovementInput (Transformation|GetActorRightVector) (Variables|Default|GetStrafe%20Value) false))

(event EventBeginPlay
  ;[1 0.06771 0.06771] Event Begin Play
  (Utilities|FlowControl|Sequence
    (:then_0
      ;;[1 1 1] Initialize AI
      (AI|RunBehaviorTree (AI|GetAIController self) "/Game/AI/BT_EnemyAI.BT_EnemyAI")
      ;;[1 1 1] set target
      (bind _returnvalue (Actor|GetActorOfClass "/Game/BaseRoll/BP_BaseRoll.BP_BaseRoll_C"))
      (bind _output_get (Variables|Default|SetTarget _returnvalue))
      (AI|Components|Blackboard|SetValueasObject (AI|GetBlackboard 0) (Utilities|Name|MakeLiteralName "Target") _output_get))
    (:then_1
      ;;[1 1 1] Defense //// wtf random defense stance - change the defense system into sth with a brain
      (Utilities|Time|SetTimerbyEvent (delegate Custom|SetDefense) (Math|Random|RandomFloatinRange 1e+01 2e+01) true))
    (:then_2
      ;;[1 1 1] Strafe / Walk sideways
      (Utilities|Time|SetTimerbyEvent (delegate Custom|SetStrafe) (Math|Random|RandomFloatinRange 1e+01 2e+01) true))
    (:then_3
      ;;[1 1 1] Sprecial attack trigger
      (Utilities|Time|SetTimerbyEvent (delegate Custom|SpecialAttack) (Math|Random|RandomFloatinRange 1e+01 3e+01) true))))

(event EventReady
  ;[1 1 1] Combat trigger
  (|Equipandreadytofight))

(fn ConstructionScript)